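; BP_Tool is an interactable tool pickup that appears as either a scalpel (Bisturi) or a pistol (Pistola).
; At BeginPlay it caches both meshes and their visibility in parallel arrays.
; Interact starts the EquipAnim timeline, which lerps the actor from its current transform toward the target and destroys it when finished.
; It also returns the first mesh recorded as visible to the caller.
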(event Custom|Interaction
  (params (Target%20Transform :type Transform))
  (bind (_location _rotation) (Math|Transform|BreakTransform Target%20Transform))
  (bind _locationcoefficinet (Timeline|Equip%20anim PlayFromStart)
    (:Update
      (Transformation|SetActorLocationAndRotation (Math|Vector|Lerp(Vector) (Transformation|GetActorLocation) _location _locationcoefficinet) (Math|Rotator|Lerp(Rotator) (Transformation|GetActorRotation) _rotation _locationcoefficinet true)))
    (:Finished
      (Actor|DestroyActor))))

(event EventBeginPlay
  (bind _bisturi (Variables|Default|Getbisturi))
  (bind _pistola (Variables|Default|Getpistola))
  (Variables|Default|SetToolVisibilityBoolean (Utilities|Array|MakeArray (Rendering|IsVisible _bisturi) (Rendering|IsVisible _pistola)))
  (Variables|Default|SetToolMeshList (Utilities|Array|MakeArray _bisturi _pistola)))

(fn ConstructionScript)

(fn Interact
  (params (Target%20Transform :type Transform))
  (CallFunction|Interaction Target%20Transform)
  (return (Utilities|Array|Get(acopy) (Variables|Default|GetToolMeshList) (Utilities|Array|FindItem (Variables|Default|GetToolVisibilityBoolean) true))))