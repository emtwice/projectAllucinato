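; Main menu HUD that takes the player from a splash screen through the menu into a dialog-punctuated intro sequence.
; Splash removal shows the menu and enables clicks; the pill reference's click event clears it and starts LS_Intro_new.
; Dialog events, not called in this graph, show widgets whose callbacks resume playback to set frames using PlayTo.
; The third dialog's callback only removes its widget; the gameplay map load is unconnected, with an empty level name.
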(event Custom|removeSplash
  ;[0.15 0.15 0.15 0.5] Splash removing and Main Menu adding
  (Widget|RemovefromParent (Variables|Default|GetSplashScreen))
  (bind _returnvalue (UserInterface|CreateWidget "/Game/Matteo/UI/WB_MainMenu.WB_MainMenu_C"))
  (bind _output_get (Variables|Default|SetMainMenu _returnvalue))
  (UserInterface|Viewport|AddtoViewport _output_get 0)
  (Variables|/Script/Engine.PlayerController|SetbEnableClickEvents (Game|GetPlayerController 0) true)
  (EventDispatchers|BindEventtoPlayClicked (Utilities|ResolveSoftReference (Variables|Default|GetPillRef)) (delegate Custom|PlayIntro)))

(event Custom|PlayIntro
  (bind _returnvalue (Game|GetPlayerController 0))
  ;[0.15 0.15 0.15 0.5] Remove main menu and play pill taken sequence
  (Variables|/Script/Engine.PlayerController|SetbEnableClickEvents _returnvalue false)
  (Variables|/Script/Engine.PlayerController|SetbShowMouseCursor _returnvalue false)
  (Utilities|FlowControl|Delay 0.5)
  (Widget|RemovefromParent (Variables|Default|GetMainMenu))
  (bind _returnvalue_2 (Sequencer|Player|CreateLevelSequencePlayer "/Game/Matteo/MainMenuCore/LS_Intro_new.LS_Intro_new"))
  (bind _output_get (Variables|Default|SetIntroSeq _returnvalue_2))
  (Class|MovieSceneSequencePlayer|Playto _output_get (Utilities|Struct|MakeMovieSceneSequencePlaybackParams (Utilities|Struct|MakeFrameTime (Utilities|Struct|MakeFrameNumber 151) 0.0) 0.0 "" "(Hours=0,Minutes=0,Seconds=0,Frames=0,Subframe=0.000000,bDropFrameFormat=False)" "Frame" "Play")))

(event Custom|GoToDoors
  ;[0.15 0.15 0.15 0.5] Resume seuqnce after dialog 2
  (Widget|RemovefromParent (Variables|Default|Getdialog2WB))
  (Class|MovieSceneSequencePlayer|Playto (Variables|Default|GetIntroSeq) (Utilities|Struct|MakeMovieSceneSequencePlaybackParams (Utilities|Struct|MakeFrameTime (Utilities|Struct|MakeFrameNumber 420) 0.0) 0.0 "" "(Hours=0,Minutes=0,Seconds=0,Frames=0,Subframe=0.000000,bDropFrameFormat=False)" "Frame" "Play")))

(event Custom|SequenceEnd
  ;[0.15 0.15 0.15 0.5] Resume sequence after dialog 3
  (Widget|RemovefromParent (Variables|Default|GetDialog3WB)))

(event Custom|GoToDialog2
  ;[0.15 0.15 0.15 0.5] Resume sequence after dialog 1
  (Widget|RemovefromParent (Variables|Default|Getdialog1WB))
  (Class|MovieSceneSequencePlayer|Playto (Variables|Default|GetIntroSeq) (Utilities|Struct|MakeMovieSceneSequencePlaybackParams (Utilities|Struct|MakeFrameTime (Utilities|Struct|MakeFrameNumber 181) 0.0) 0.0 "" "(Hours=0,Minutes=0,Seconds=0,Frames=0,Subframe=0.000000,bDropFrameFormat=False)" "Frame" "Play")))

(event EventBeginPlay
  (bind _returnvalue (Game|GetPlayerController 0))
  (Utilities|FlowControl|Sequence
    (:then_0
      ;[0.15 0.15 0.15 0.5] SplashScreen creation
      (bind _returnvalue_2 (UserInterface|CreateWidget "/Game/Matteo/UI/WB_SplashScreen.WB_SplashScreen_C"))
      (bind _output_get (Variables|Default|SetSplashScreen _returnvalue_2))
      (UserInterface|Viewport|AddtoViewport _output_get 0)
      (Input|SetInputModeGameandUI _returnvalue 0 "DoNotLock" true false)
      (Variables|/Script/Engine.PlayerController|SetbShowMouseCursor _returnvalue true))
    (:then_1
      ;[0.15 0.15 0.15 0.5] Splash removing and Main Menu adding
      (EventDispatchers|BindEventtoRemovedSplashScreen (Variables|Default|GetSplashScreen) (delegate Custom|removeSplash)))))

(event EventDialog3
  ;[0.15 0.15 0.15 0.5] Resume sequence after dialog 3
  (bind _returnvalue (UserInterface|CreateWidget "/Game/Matteo/UI/WB_Dialog3.WB_Dialog3_C"))
  (bind _output_get (Variables|Default|SetDialog3WB _returnvalue))
  (UserInterface|Viewport|AddtoViewport _output_get 0)
  (Variables|/Script/Engine.PlayerController|SetbShowMouseCursor (Game|GetPlayerController 0) true)
  (EventDispatchers|BindEventtoSequenceEnd (Variables|Default|GetDialog3WB) (delegate Custom|SequenceEnd)))

(event EventDialog1
  ;[0.15 0.15 0.15 0.5] Resume sequence after dialog 1
  (bind _returnvalue (UserInterface|CreateWidget "/Game/Matteo/UI/WB_Dialog1.WB_Dialog1_C"))
  (bind _output_get (Variables|Default|Setdialog1WB _returnvalue))
  (UserInterface|Viewport|AddtoViewport _output_get 0)
  (Variables|/Script/Engine.PlayerController|SetbShowMouseCursor (Game|GetPlayerController 0) true)
  (EventDispatchers|BindEventtoGotoDialog1 (Variables|Default|Getdialog1WB) (delegate Custom|GoToDialog2)))

(event EventDialog2
  ;[0.15 0.15 0.15 0.5] Resume seuqnce after dialog 2
  (bind _returnvalue (UserInterface|CreateWidget "/Game/Matteo/UI/WB_Dialog2.WB_Dialog2_C"))
  (bind _output_get (Variables|Default|Setdialog2WB _returnvalue))
  (UserInterface|Viewport|AddtoViewport _output_get 0)
  (Variables|/Script/Engine.PlayerController|SetbShowMouseCursor (Game|GetPlayerController 0) true)
  (EventDispatchers|BindEventtoGotoDoors (Variables|Default|Getdialog2WB) (delegate Custom|GoToDoors)))

(fn ConstructionScript)