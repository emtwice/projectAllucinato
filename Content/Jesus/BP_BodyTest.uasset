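; BP_BodyTest is a test body actor that holds a life value and exposes its Bones and Skin through getters.
; BeginPlay stores the starting Life as MaxLife and starts a looping timer through a created event delegate, whose target is not shown.
; SubtractLife lowers Life, clamped between zero and MaxLife, and prints the result.
; CallLessLife applies a fixed amount of damage through SubtractLife.
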(event Custom|CallLessLife
  (CallFunction|SubtractLife 30))

(event EventBeginPlay
  (Variables|Default|SetMaxLife (Variables|Default|GetLife))
  (Utilities|Time|SetTimerbyEvent (EventDispatchers|CreateEvent :!event Custom|CallLessLife) 3.0 true))

(event Collision|EventActorBeginOverlap
  (params (OtherActor :type Actor%20Object%20Reference)))

(event EventTick
  (params (DeltaSeconds :type Float%20%28single-precision%29)))

(event EventSubtractLife
  (params (LifeToSubstrac :type Integer))
  (bind _output_get (Variables|Default|SetLife (Math|Integer|Clamp(Integer) (- (Variables|Default|GetLife) LifeToSubstrac) 0 (Variables|Default|GetMaxLife))))
  (Development|PrintString (Utilities|String|Append "life is " (Utilities|String|ToString(Integer) _output_get))))

(fn ConstructionScript)

(fn GetBones
  (return (Variables|Default|GetBones)))

(fn GetSkin
  (return (Variables|Default|GetSkin)))