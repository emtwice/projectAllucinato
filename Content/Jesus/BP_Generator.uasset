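; BP_Generator is a procedural level generator that spawns a random starting room, then recursively attaches more random rooms.
; Each pass pools the last room's BP_ParentLevel exits and randomly tries rooms at open exits until one fits.
; Overlapping rooms are destroyed via their OverlapCheck component.
; The exit's door meshes are then hidden and made non-colliding, the exit leaves the pool, and RoomCounter limits the recursion.
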(event Custom|SpawnRoom
  ;[0.15 0.15 0.15 0.5] Get the previous room and access child info thanks to the father. In this way, we can get all exits of the room.
  ;;[0.15 0.15 0.15 0.5] If Ref change must change the interface output
  (bind _asbp_parent_level (Utilities|Casting|CastToBP_ParentLevel (Variables|Default|GetLastRoom)))
  (for _array_element (Components|GetChildrenComponents (Variables|/Game/Jesus/BP_ParentLevel.BP_ParentLevel_C|GetExists _asbp_parent_level) false)
    (if (not (Utilities|Array|ContainsItem (Variables|Default|GetLastExists) _array_element))
      (Utilities|Array|Add (Variables|Default|GetLastExists) _array_element)))
  ;[0.15 0.15 0.15 0.5] Random calcolate the % of spawn a room for each exit
  (bind _array_element_2 (Utilities|Array|ForEachLoopwithBreak (Variables|Default|GetLastExists) :!label _label)
    (:LoopBody
      (if (< (Math|Random|RandomInteger 100) 50)
        ;[0.15 0.15 0.15 0.5] Spawn Random Room in the exit position
        (bind _returnvalue (Game|SpawnActorfromClass (.OutItem (Utilities|Array|Random (Variables|Default|GetRooms))) (Math|Transform|MakeTransform (Transformation|GetWorldLocation _array_element_2) (Transformation|GetWorldRotation _array_element_2) "1.000000,1.000000,1.000000") "AlwaysSpawn" "MultiplyWithRoot" 0 0))
        ;[0.15 0.15 0.15 0.5] If there is another room in the same position delete the last one
        (bind _generate_ (CallFunction|CheckCollisionF _returnvalue))
        (if _generate_
          (Variables|Default|SetLastRoom _returnvalue)
          (goto _label Break))))
    (:Completed
      (CallFunction|OpenDoors _array_element_2)
      (Utilities|Array|RemoveItem (Variables|Default|GetLastExists) _array_element_2)
      ;[0.15 0.15 0.15 0.5] if spawn a room reduce the room counter. if counter is fill do nothing if not call recursive spawn function
      (Math|Integer|DecrementInt (Variables|Default|GetRoomCounter)
        (:%20%20
          (bind _output_get (Variables|Default|SetRoomCounter (Variables|Default|GetRoomCounter)))
          (if (> _output_get 0)
            (CallFunction|SpawnRoom)))))))

(event EventBeginPlay
  ;[0.15 0.15 0.15 0.5] Just spawn the starting room. it can be random
  (bind _returnvalue (Game|SpawnActorfromClass (.OutItem (Utilities|Array|Random (Variables|Default|GetRooms))) (Math|Transform|MakeTransform "0, 0, 0" "0, 0, 0" "1.000000,1.000000,1.000000") "AlwaysSpawn" "MultiplyWithRoot" 0 0))
  (Variables|Default|SetLastRoom _returnvalue)
  (CallFunction|SpawnRoom))

(fn ConstructionScript)

(fn CheckCollisionF
  (params (CurrentRoom :type Actor%20Object%20Reference))
  ;[0.15 0.15 0.15 0.5] Check if collide with another level
  (bind _asbp_parent_level (Utilities|Casting|CastToBP_ParentLevel CurrentRoom))
  (if (Utilities|Array|IsNotEmpty (Class|PrimitiveComponent|GetOverlappingComponents (Variables|/Game/Jesus/BP_ParentLevel.BP_ParentLevel_C|GetOverlapCheck _asbp_parent_level)))
    ;[0.15 0.15 0.15 0.5] Destroy the last room created
    (Actor|DestroyActor CurrentRoom)
    (return false)
    (else
      (return true))))

(fn OpenDoors
  (params (ExitRef :type Scene%20Component%20Object%20Reference))
  (for _array_element (Components|GetChildrenComponents ExitRef false)
    (bind _asstatic_mesh_component (Utilities|Casting|CastToStaticMeshComponent _array_element))
    (Collision|SetCollisionResponsetoAllChannels _asstatic_mesh_component "ECR_Ignore")
    (Rendering|SetVisibility _array_element false true)))